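; BP_GM is a game manager Blueprint that starts the match and assigns the Herobrine role.
; ControlHerobrine stores a control flag and a chosen PlayerState, though StartGame recomputes the flag from that PlayerState's validity.
; StartGame spawns BP_Herobrine high above the origin with the flag, then enables movement on every Player actor.
; With a valid PlayerState, that player's controller possesses Herobrine and the old pawn is destroyed.
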(event `ControlHerobrine`
  (params (ControlHerobrineVar :type Boolean) (PlayerStateHerobrine :type "PlayerState Object Reference"))
  (set `self.ControlHerobrineVar` ControlHerobrineVar)
  (set `self.PlayerStateHerobrine` PlayerStateHerobrine))

(event `StartGame`
  (bind _playerstateherobrine (`self.PlayerStateHerobrine`)
    (:`then`
      (set `self.ControlHerobrineVar` true))
    (:`else`
      (set `self.ControlHerobrineVar` false)))
  (bind _returnvalue (`|SpawnActorFromClass` "/Game/BP_Herobrine.BP_Herobrine_C" (`KismetMathLibrary.MakeTransform` (0.0 0.0 10000.0)) "Undefined" "OverrideRootScale" null (`self.ControlHerobrineVar`) null))
  (`|ExecutionSequence`
    (:`then_0`
      (bind _outactors (`GameplayStatics.GetAllActorsOfClass` "/Game/Herobrine/NewFolder/Player.Player_C"))
      (for _array_element _outactors
        (set `/Game/Herobrine/NewFolder/Player.EnableMovement` true _array_element)))
    (:`then_1`
      (`self.PlayerStateHerobrine`
        (:`then`
          (bind _returnvalue_2 (`PlayerState.GetPawn` _playerstateherobrine))
          (set `self.deleteplayer` _returnvalue_2)
          (`Controller.Possess` (`Pawn.GetController` _returnvalue_2) _returnvalue)
          (bind _deleteplayer (`self.deleteplayer`)
            (:`then`
              (`self.K2_DestroyActor` _deleteplayer))
            (:`else`)))
        (:`else`)))))

(fn `UserConstructionScript`)