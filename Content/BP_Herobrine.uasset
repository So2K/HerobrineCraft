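; Networked Herobrine monster character that hunts players, controlled either by AI or by a player.
; As AI, the server teleports it near random players or, through PawnSensing, to unseen spots; player control adds aimed teleport and translucent sprint while unwatched.
; Its sphere overlap damages players and relocates it until enough spawned diamonds are found.
; Swords then appear, and touching it triggers its ragdoll death, clearing weather and setting the win.
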(event `ScreamSound`
  ;[1 1 1] Sounds (Multicast)
)

(event `PlaySound`
  (params (Sound :type "SoundBase Object Reference"))
  ;[1 1 1] Sounds (Multicast)
  (`GameplayStatics.PlaySound2D` Sound 3.0 1.0 0.0 null null))

(event `PlaySoundTP`
  ;[1 1 1] Sounds (Multicast)
  (`GameplayStatics.PlaySoundAtLocation` "/Game/Audio/teleportsound_Cue.teleportsound_Cue" (`self.K2_GetActorLocation`) (struct) 1.0 1.0 0.0 null null null null))

(event `TeleportRequest`
  (params (DestLocation :type "Vector Structure"))
  ;[1 1 1] Teleport Reuqest (server)
  (`/Engine/EditorBlueprintResources/StandardMacros.DoOnce` false :!label _label
    (:`Completed`
      (`SceneComponent.K2_SetWorldLocation` (`self.RootComponent`) DestLocation false false)
      (`self.PlaySoundTP`)
      (`KismetSystemLibrary.Delay` 3.0)
      (goto _label :!via `Reset`))))

(event `Key|V`
  (params (Key :type "Key Structure"))
  ;[1 1 1] TELEPORT INPUT
  (:`Pressed`
    (bind (_start _end) (`self.Linetrace_0` 5000.0))
    (bind (_outhit _returnvalue) (`KismetSystemLibrary.LineTraceSingle` _start _end "TraceTypeQuery1"))
    (if _returnvalue
      (bind (_bblockinghit _binitialoverlap _time _distance _location _impactpoint _normal _impactnormal _physmat _hitactor _hitcomponent _hitbonename _bonename _hititem _elementindex _faceindex _tracestart _traceend) (`GameplayStatics.BreakHitResult` _outhit))
      (`self.TeleportRequest` _location)
      (else
        (`self.TeleportRequest` _traceend)))))

(event `Screamer`
  (params (Player :type "/Game/Herobrine/NewFolder/Player Object Reference"))
  (bind _physicscameracomponent (`/Game/Herobrine/NewFolder/Player.PhysicsCameraComponent` Player))
  (bind (_returnvalue_roll _returnvalue_pitch _returnvalue_yaw) (`KismetMathLibrary.BreakRotator` (`SceneComponent.K2_GetComponentRotation` _physicscameracomponent)))
  (bind (_start _end) (`/Game/Herobrine/NewFolder/Player.Linetrace` Player 300.0))
  (bind _outhit (`KismetSystemLibrary.LineTraceSingle` :`Start` _start :`End` _end :`TraceChannel` "TraceTypeQuery1" :`DrawDebugType` "ForDuration"))
  (`self.K2_TeleportTo` (`.TraceEnd` (`GameplayStatics.BreakHitResult` _outhit)) (`KismetMathLibrary.MakeRotator` 0.0 0.0 (- _returnvalue_yaw 180.0)))
  (bind (_direction _newtrack_0) (`Timeline|Timeline_0` :!via `PlayFromStart`)
    (:`Update`
      (`CameraComponent.SetFieldOfView` _physicscameracomponent (* _newtrack_0 90.0)))))

(event `RandomTP`
  (bind _rootcomponent (`self.RootComponent`))
  (bind _outactors (`GameplayStatics.GetAllActorsOfClass` "/Game/SPAWNLINETRACE.SPAWNLINETRACE_C"))
  (bind (_outhit _returnvalue) (`/Game/SPAWNLINETRACE.Linetrace` (`|GetArrayItem` _outactors)))
  (if _returnvalue
    (bind (_bblockinghit _binitialoverlap _time _distance _location _impactpoint _normal _impactnormal _physmat _hitactor _hitcomponent _hitbonename _bonename _hititem _elementindex _faceindex _tracestart _traceend) (`GameplayStatics.BreakHitResult` _outhit))
    (`SceneComponent.K2_SetWorldLocation` _rootcomponent _location false true)
    (else
      (`SceneComponent.K2_SetWorldLocation` _rootcomponent _traceend false true))))

(event `ReplicateHead`
  (params (NewVar_0 :type "Rotator Structure"))
  (set `self.NewVar_0` NewVar_0))

(event `ShowSwords`
  (params (Array :type "Array of /Game/Herobrine/NewFolder/Player Object Reference"))
  ;[0.2451 1 0.01415] Show Swords (Multicast)
  (for _array_element Array
    (`SceneComponent.SetVisibility` (`/Game/Herobrine/NewFolder/Player.Sword` _array_element) true false)))

(event `DEATH HEROBRINE`
  (bind _mesh (`self.Mesh`))
  (`PrimitiveComponent.SetCollisionEnabled` _mesh "QueryAndPhysics")
  (`PrimitiveComponent.SetSimulatePhysics` _mesh true)
  (`SkeletalMeshComponent.BreakConstraint` _mesh (50.0 0.0 0.0) (`SceneComponent.K2_GetComponentLocation` _mesh) "Peito")
  (set `self.Death` true)
  (bind _returnvalue (`PrimitiveComponent.CreateDynamicMaterialInstance` _mesh 0 "/Game/Herobrine/NewFolder/NewMaterial.NewMaterial" "None"))
  (`MaterialInstanceDynamic.SetScalarParameterValue` _returnvalue "Intensity" 0.0)
  (bind _outactors (`GameplayStatics.GetAllActorsOfClass` "/Game/UltraDynamicSky/Blueprints/Ultra_Dynamic_Weather.Ultra_Dynamic_Weather_C"))
  (`/Game/UltraDynamicSky/Blueprints/Ultra_Dynamic_Weather.Change Weather` (`|GetArrayItem` _outactors) "/Game/UltraDynamicSky/Blueprints/Weather_Effects/Weather_Presets/Clear_Skies.Clear_Skies" 10.0 false)
  (bind _outactors_2 (`GameplayStatics.GetAllActorsOfClass` "/Game/UltraDynamicSky/Blueprints/Ultra_Dynamic_Sky.Ultra_Dynamic_Sky_C"))
  (set `/Game/UltraDynamicSky/Blueprints/Ultra_Dynamic_Sky.Animate Time of Day` true (`|GetArrayItem` _outactors_2))
  (bind (_direction _newtrack_0) (`Timeline|roughness` :!via `PlayFromStart`)
    (:`Update`
      (`KismetMaterialLibrary.SetScalarParameterValue` "/Game/Herobrine/NewFolder/NewMaterialParameterCollection.NewMaterialParameterCollection" "Roughness" _newtrack_0))))

(event `FoundDiamond`
  ;[1 0.151 0.151] Found Diamond (Server)
  (bind _result (`/Engine/EditorBlueprintResources/StandardMacros.IncrementInt` (`self.FoundDiamonds`))
    (:`  `
      (`self.ForceNetUpdate`)
      (if (== (`self.NeedFindDiamonds`) _result)
        (set `self.FindDiamonds` true)
        (bind _outactors (`GameplayStatics.GetAllActorsOfClass` "/Game/Herobrine/NewFolder/Player.Player_C"))
        (`self.ShowSwords` _outactors)
        (`SphereComponent.SetSphereRadius` (`self.Sphere`) 8.0 true)))))

(event `PlaySoundServer`
  (`self.PlaySound` (select `int` (`KismetMathLibrary.RandomIntegerInRange` 0 6) :`0` "/Game/Audio/cave1.cave1" :`1` "/Game/Audio/cave2.cave2" :`2` "/Game/Audio/cave5.cave5" :`3` "/Game/Audio/cave6.cave6" :`4` "/Game/Audio/cave10.cave10" :`5` "/Game/Audio/cave14.cave14" :`6` "/Game/Audio/cave19.cave19" :`7` null :!type "SoundBase Object Reference")))

(event `self.ReceiveTick`
  (params (DeltaSeconds :type "Float (single-precision)"))
  (bind (_returnvalue_roll _returnvalue_pitch _returnvalue_yaw) (`KismetMathLibrary.BreakRotator` (`self.K2_GetActorRotation`)))
  (bind (_returnvalue_roll_2 _returnvalue_pitch_2 _returnvalue_yaw_2) (`KismetMathLibrary.BreakRotator` (`self.GetControlRotation`)))
  (bind _returnvalue (`KismetMathLibrary.MakeRotator` (- 0.0 _returnvalue_pitch_2) 0.0 (`KismetMathLibrary.ClampAngle` (- _returnvalue_yaw_2 _returnvalue_yaw) -179.0 180.0)))
  (`|ExecutionSequence`
    (:`then_0`
      (if (`KismetSystemLibrary.IsServer`)
        (`|ExecutionSequence`
          (:`then_0`
            ;[1 1 1] Random Scream
            (`KismetSystemLibrary.Delay` (`KismetMathLibrary.RandomFloatInRange` 10.0 60.0))
            (bind _outactors (`GameplayStatics.GetAllActorsOfClass` "/Game/BP_Scream.BP_Scream_C"))
            (`/Game/BP_Scream.PlaySound` (`KismetArrayLibrary.Array_Random` _outactors))
            (`KismetSystemLibrary.PrintString` "SCREEEEEEEAM"))
          (:`then_1`
            (if (not (`self.Player`))
              (`KismetSystemLibrary.Delay` (`KismetMathLibrary.RandomFloatInRange` 2.0 15.0))
              (bind _outactors_2 (`GameplayStatics.GetAllActorsOfClass` "/Game/Herobrine/NewFolder/Player.Player_C"))
              (`self.SpawnNearPlayer` (`KismetArrayLibrary.Array_Random` _outactors_2)))))))
    (:`then_1`
      (if (`self.IsLocallyControlled`)
        (if (`self.Player`)
          (`self.ReplicateHead` _returnvalue)
          (set `self.NewVar_0` _returnvalue))))))

(event `SpawnNearPlayer`
  (params (Target :type "Actor Object Reference"))
  (bind _returnvalue (`KismetMathLibrary.RandomBool`))
  (bind _returnvalue_2 (`KismetMathLibrary.SelectFloat` (+ 0.0 -2000.0) (+ 0.0 2000.0) _returnvalue))
  (bind _returnvalue_3 (`KismetMathLibrary.SelectFloat` (+ -500.0 0.0) (+ 0.0 500.0) _returnvalue))
  (bind _returnvalue_4 (+ (`self.K2_GetActorLocation` Target) (`KismetMathLibrary.MakeVector` (`KismetMathLibrary.RandomFloatInRange` _returnvalue_3 _returnvalue_2) (`KismetMathLibrary.RandomFloatInRange` _returnvalue_3 _returnvalue_2) (select `bool` (`/Game/BP_GM.Building` (cast `/Game/BP_GM` (`GameplayStatics.GetGameMode`) :!pure true)) :`false` 3000.0 :`true` 50.0))))
  (bind (_outhit _returnvalue_5) (`KismetSystemLibrary.LineTraceSingle` :`Start` _returnvalue_4 :`End` (+ _returnvalue_4 (* (`self.GetActorUpVector` Target) -10000.0)) :`TraceChannel` "TraceTypeQuery1" :`bTraceComplex` true :`DrawDebugType` "ForDuration"))
  (if _returnvalue_5
    (`self.SETWORLDLOCATION` (`.Location` (`GameplayStatics.BreakHitResult` _outhit)) (`self.K2_GetActorLocation`) (`KismetMathLibrary.RandomBoolWithWeight` 0.8))))

(event `SETWORLDLOCATION`
  (params (NewLocation :type "Vector Structure") (OldLocation :type "Vector Structure") (NoSound :type Boolean))
  ;[0.2921 1 0.3274] SETWORLDLOCATION (MULTICAST)
  (`SceneComponent.K2_SetWorldLocation` (`self.RootComponent`) NewLocation false true)
  (if (not NoSound)
    (`GameplayStatics.PlaySoundAtLocation` "/Game/Audio/teleportsound_Cue.teleportsound_Cue" NewLocation (struct) 1.0 1.0 0.0 null null null null)
    (`GameplayStatics.PlaySoundAtLocation` "/Game/Audio/teleportsound_Cue.teleportsound_Cue" OldLocation (struct) 1.0 1.0 0.0 null null null null)))

(event `TPBEHINDPLAYER`
  ;[1 0.5885 0.5885] TP Behind Player (NPC) (Dont see) (Server)
  (bind (_start _end) (`self.Linetrace` 500.0))
  (bind _outhit (`KismetSystemLibrary.LineTraceSingle` :`Start` _start :`End` _end :`TraceChannel` "TraceTypeQuery1" :`DrawDebugType` "ForDuration"))
  (`self.SETWORLDLOCATION` (`.TraceEnd` (`GameplayStatics.BreakHitResult` _outhit)) (`self.K2_GetActorLocation`) (`KismetMathLibrary.RandomBoolWithWeight` 0.8)))

(event `self.ReceiveBeginPlay`
  ;[1 0.1354 0.1354] Event BeginPlay (Server)
  (`/Engine/EditorBlueprintResources/ActorMacros.Switch Has Authority`
    (:`Authority`
      (`KismetSystemLibrary.Delay` 0.2)
      (bind _outactors (`GameplayStatics.GetAllActorsOfClass` "/Game/Creppy/Diamond/BP_DiamondSpawn.BP_DiamondSpawn_C"))
      (bind _output_get (set `self.Out Actors` _outactors))
      (`KismetArrayLibrary.Array_Shuffle` _output_get)
      (bind _outactors_2 (`GameplayStatics.GetAllActorsOfClass` "/Game/Herobrine/NewFolder/Player.Player_C"))
      (bind _returnvalue (`KismetMathLibrary.Clamp` (* (`KismetArrayLibrary.Array_Length` _outactors_2) 15) 5 25))
      (for _index (range 1 (+ _returnvalue 1))
        (bind (_returnvalue_location _returnvalue_rotation) (`KismetMathLibrary.BreakTransform` (`self.GetTransform` (`|GetArrayItem` (`self.Out Actors`) _index))))
        (`|SpawnActorFromClass` "/Game/Creppy/Diamond/BP_Diamond.BP_Diamond_C" (`KismetMathLibrary.MakeTransform` _returnvalue_location _returnvalue_rotation (0.1 0.1 0.1)) "AlwaysSpawn" "OverrideRootScale" null self null))
      (set `self.NeedFindDiamonds` 25)
      (`KismetSystemLibrary.PrintString` (`KismetStringLibrary.Conv_IntToString` _returnvalue))
      (if (`self.Player`)
        (`SphereComponent.SetSphereRadius` (`self.Sphere`) 15.0 false)))))

(event `Opacity`
  (params (NewParam :type Boolean))
  (bind _mesh (`self.Mesh`))
  (if NewParam
    (`PrimitiveComponent.SetMaterial` _mesh 0 "/Game/Herobrine/NewFolder/herobrineopacity.herobrineopacity")
    (else
      (`PrimitiveComponent.SetMaterial` _mesh 0 "/Game/Herobrine/NewFolder/NewMaterial.NewMaterial"))))

(event `Sprint`
  (params (Sprint :type Boolean))
  (if (`self.ViewedByPlayer?`)
    _
    (elif Sprint
      (set `self.speed` 1500.0)
      (`self.Opacity` true)
      (else
        (set `self.speed` 600.0)
        (`self.Opacity` false)))))

(event `Key|LeftShift`
  (params (Key :type "Key Structure"))
  ;[1 1 1] INPUT
  (:`Pressed`
    (`self.Sprint` true))
  (:`Released`
    (`self.Sprint` false)))

(event `ViewPlayer`
  (params (Visible :type Boolean))
  (`KismetSystemLibrary.PrintString` (`KismetStringLibrary.Conv_BoolToString` Visible) true true (struct :`R` 0.249851 :`G` 1.0 :`A` 1.0))
  (bind _output_get (set `self.ViewedByPlayer?` Visible))
  (if _output_get
    (set `self.speed` 600.0)
    (`self.Opacity` false)))

(event `InputAction|Jump` :overrideparent false
  (params (Key :type "Key Structure"))
  ;[1 1 1] INPUT
  (:`Pressed`
    (`self.Jump`))
  (:`Released`
    (`self.StopJumping`)))

(event `InputAxis|MoveForward` :consume false :overrideparent false
  (params (AxisValue :type "Float (single-precision)"))
  (bind (_returnvalue_roll _returnvalue_pitch _returnvalue_yaw) (`KismetMathLibrary.BreakRotator` (`self.GetControlRotation`)))
  (bind _charactermovement (`self.CharacterMovement`))
  ;[1 1 1] INPUT
  (if (or (`NavMovementComponent.IsFlying` _charactermovement) (`NavMovementComponent.IsSwimming` _charactermovement))
    (`self.AddMovementInput` (`KismetMathLibrary.GetForwardVector` (`KismetMathLibrary.MakeRotator` _returnvalue_roll _returnvalue_pitch _returnvalue_yaw)) AxisValue)
    (else
      (`self.AddMovementInput` (`self.GetActorForwardVector`) AxisValue))))

(event `InputAxis|MoveRight` :consume false :overrideparent false
  (params (AxisValue :type "Float (single-precision)"))
  ;[1 1 1] INPUT
  (`self.AddMovementInput` (`self.GetActorRightVector`) AxisValue))

(event `InputAxis|Turn` :overrideparent false
  (params (AxisValue :type "Float (single-precision)"))
  ;[1 1 1] INPUT
  (`self.AddControllerYawInput` AxisValue))

(event `InputAxis|LookUp` :overrideparent false
  (params (AxisValue :type "Float (single-precision)"))
  ;[1 1 1] INPUT
  (`self.AddControllerPitchInput` AxisValue))

(event `CANSEEPLAYER?`
  (params (Pawn :type "Pawn Object Reference"))
  ;[1 0.4479 0.4479] Can See Player? Server (NPC)
  (bind _asplayer (cast `/Game/Herobrine/NewFolder/Player` Pawn))
  (if (not (`/Game/Herobrine/NewFolder/Player.SEE` _asplayer))
    (`/Engine/EditorBlueprintResources/StandardMacros.DoOnce` false :!label _label_2
      (:`Completed`
        (`self.TPBEHINDPLAYER`)
        (`KismetSystemLibrary.Delay` 0.2)
        (goto _label_2 :!via `Reset`)))))

(event `self.PawnSensing.OnSeePawn`
  (params (Pawn :type "Pawn Object Reference"))
  ;[1 1 1] On See Pawn (Server)
  (`/Engine/EditorBlueprintResources/ActorMacros.Switch Has Authority`
    (:`Authority`
      (if (not (`self.Player`))
        (`self.Hear` Pawn)
        (`self.CANSEEPLAYER?` Pawn)))))

(event `Hear`
  (params (Pawn :type "Pawn Object Reference"))
  ;[0.7287 0.5975 1] Head Rotation (Server) (NPC)
  (cast `/Game/Herobrine/NewFolder/Player` Pawn)
  (set `self.NewVar_0` (`KismetMathLibrary.FindLookAtRotation` (`self.K2_GetActorLocation`) (`self.K2_GetActorLocation` Pawn))))

(event `self.PawnSensing.OnHearNoise`
  (params (Instigator :type "Pawn Object Reference") (Location :type "Vector Structure (by ref)") (Volume :type "Float (single-precision)"))
  ;[1 1 1] On Hear Noise (Server)
  (`/Engine/EditorBlueprintResources/ActorMacros.Switch Has Authority`
    (:`Authority`
      (if (not (`self.Player`))
        (cast `/Game/Herobrine/NewFolder/Player` Instigator)
        (`self.Hear` Instigator)
        (`self.CANSEEPLAYER?` Instigator)))))

(event `self.Sphere.OnComponentBeginOverlap`
  (params (OverlappedComponent :type "PrimitiveComponent Object Reference") (OtherActor :type "Actor Object Reference") (OtherComp :type "PrimitiveComponent Object Reference") (OtherBodyIndex :type Integer) (bFromSweep :type Boolean) (SweepResult :type "HitResult Structure (by ref)"))
  ;[0.2396 0.9123 1] Damage Zone (Server)
  (`/Engine/EditorBlueprintResources/ActorMacros.Switch Has Authority`
    (:`Authority`
      (bind _asplayer (cast `/Game/Herobrine/NewFolder/Player` OtherActor))
      (if (`self.FindDiamonds`)
        (`self.DEATH HEROBRINE`)
        (`KismetSystemLibrary.Delay` 3.0)
        (set `self.Win` true)
        (else
          (`/Engine/EditorBlueprintResources/StandardMacros.DoOnce` false :!label _label_3
            (:`Completed`
              (`/Game/Herobrine/NewFolder/Player.HurtUI` _asplayer)
              (`self.ScreamSound`)
              (`GameplayStatics.ApplyDamage` _asplayer 1.0)
              (`self.RandomTP`)
              (`KismetSystemLibrary.Delay` 1.0)
              (goto _label_3 :!via `Reset`))))))))

(fn `Linetrace`
  (params (Distance :type "Float (double-precision)"))
  (returns (Start :type "Vector Structure") (End :type "Vector Structure"))
  (bind _physicscameracomponent (`self.PhysicsCameraComponent`))
  (bind _returnvalue (`SceneComponent.K2_GetComponentLocation` _physicscameracomponent))
  (return _returnvalue (+ _returnvalue (* (`SceneComponent.GetForwardVector` _physicscameracomponent) Distance))))

(fn `Linetrace_0`
  (params (Distance :type "Float (double-precision)"))
  (returns (Start :type "Vector Structure") (End :type "Vector Structure"))
  (bind _arrow1 (`self.Arrow1`))
  (bind _returnvalue (`SceneComponent.K2_GetComponentLocation` _arrow1))
  (return _returnvalue (+ _returnvalue (* (`SceneComponent.GetForwardVector` _arrow1) Distance))))

(fn `OnRep_speed`
  (set `CharacterMovementComponent.MaxWalkSpeed` (`self.speed`) (`self.CharacterMovement`)))

(fn `OnRep_Torch`)

(fn `UserConstructionScript`)